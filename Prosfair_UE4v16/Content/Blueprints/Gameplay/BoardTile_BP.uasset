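; BoardTile_BP is a game board tile actor that comes in a light or dark polished marble look.
; The construction script picks the Tile material from TileColor.
; On BeginPlay it stores the first GamePiece_BP overlapping its CollisionBox as CurrentGamePiece.
; Clicking the tile only prints its object name to the screen.
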(event EventBeginPlay
  (for (_array_element _array_index) (Collision|GetOverlappingActors (Variables|Default|GetCollisionBox) "/Game/Blueprints/GamePieces/GamePiece_BP.GamePiece_BP_C" :!class /Script/Engine.PrimitiveComponent)
    (if (== _array_index 0)
      (bind _asgame_piece_bp (Utilities|Casting|CastToGamePiece_BP _array_element))
      (Variables|Default|SetCurrentGamePiece _asgame_piece_bp))))

(event MouseInput|EventActorOnClicked
  (params (ButtonPressed :type Key%20Structure :default "AnyKey"))
  (Development|PrintString (Utilities|GetObjectName self) true true "(R=0.000000,G=0.660000,B=1.000000,A=1.000000)" 5.0))

(fn ConstructionScript
  (bind _tile (Variables|Default|GetTile))
  (if (Utilities|Enum|Equal(Enum) (Variables|Default|GetTileColor) "Light")
    (Rendering|Material|SetMaterial _tile 0 "/Game/Materials/Board/M_Rock_Marble_Polished_LightInst.M_Rock_Marble_Polished_LightInst")
    (else
      (Rendering|Material|SetMaterial _tile 0 "/Game/Materials/Board/M_Rock_Marble_Polished_DarkInst.M_Rock_Marble_Polished_DarkInst"))))