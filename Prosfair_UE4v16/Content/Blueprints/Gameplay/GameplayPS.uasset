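; GameplayPS is the gameplay player state, holding a player's number and faction.
; On BeginPlay it caches the GameplayGS game state, calls its AssignPlayerNumber, then sets a temporary faction that differs for player 0 versus all others.
; SetPlayerController is an empty stub, and the nodes that would cache the GameplayPC controller are disconnected and never run.
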(event Custom|SetPlayerController
  (params (PlayerController :type Gameplay%20PC%20Object%20Reference)))

(event EventBeginPlay
  ;[1 1 1] Begin Play
  (bind _asgameplay_gs (Utilities|Casting|CastToGameplayGS (Game|GetGameState)))
  (bind _output_get (Variables|Default|SetgameState _asgameplay_gs))
  (Default|AssignPlayerNumber _output_get)
  ;[1 1 1] Temporary Faction Assignment
  (if (== (Variables|Default|GetplayerNumber) 0)
    (Variables|Default|SetplayerFaction "NewEnumerator1")
    (else
      (Variables|Default|SetplayerFaction "NewEnumerator0"))))

(fn ConstructionScript)