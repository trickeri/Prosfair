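; Game state for a two-player, turn-based board game that assigns player numbers, switches turns and moves pieces between tiles.
; Players get number 0 or 1 by alternating PlayerArray index.
; Turn and move events forward to Multi counterparts that flip PlayerTurn or relocate the selected tile's piece.
; Moves find the destination by object name among tiles cached at construction, clear selection, then have every tile recheck for pieces.
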(event Custom|AssignPlayerNumber
  ;[1 1 1] Assigning Player Number
  (for (_array_element _array_index) (Variables|Default|GetPlayerArray)
    (if (== (Math|Integer|%(Integer) _array_index 2) 0)
      (bind _asgameplay_ps (Utilities|Casting|CastToGameplayPS _array_element))
      (Variables|/Game/Blueprints/Gameplay/GameplayPS.GameplayPS_C|SetplayerNumber _asgameplay_ps 0)
      (else
        (bind _asgameplay_ps_2 (Utilities|Casting|CastToGameplayPS _array_element))
        (Variables|/Game/Blueprints/Gameplay/GameplayPS.GameplayPS_C|SetplayerNumber _asgameplay_ps_2 1)))))

(event Custom|MovePiece_GS_Multi
  (params (TileMovingTo :type String) (CurrentlySelectedTile :type Board%20Tile%20BP%20Object%20Reference))
  (bind _allboardtiles (Variables|Default|GetallBoardTiles))
  (bind _array_element (Utilities|Array|ForEachLoopwithBreak _allboardtiles :!label _label)
    (:LoopBody
      (if (Utilities|Enum|Equal(Enum) TileMovingTo (Utilities|GetObjectName _array_element))
        (Transformation|SetActorLocation (Variables|/Game/Blueprints/Gameplay/BoardTile_BP.BoardTile_BP_C|GetCurrentGamePiece CurrentlySelectedTile) (Transformation|GetActorLocation _array_element) false false)
        (Default|SetOriginalTileColor CurrentlySelectedTile)
        (bind _asgameplay_pc (Utilities|Casting|CastToGameplayPC (Game|GetPlayerController 0)))
        (Variables|/Game/Blueprints/Gameplay/GameplayPC.GameplayPC_C|SetpieceIsSelected _asgameplay_pc false)
        (goto _label Break)))
    (:Completed
      (for _array_element_2 _allboardtiles
        (Default|CheckforGamePiece _array_element_2)))))

(event Custom|EndPlayerTurn
  (params (previousPlayerTurn :type Integer))
  ;[1 1 1] Switch Player Turn
  (CallFunction|EndPlayerTurnMulti previousPlayerTurn))

(event Custom|EndPlayerTurn_Multi
  (params (previousPlayerTurn :type Integer))
  ;[1 1 1] Switch Player Turn
  (switch int previousPlayerTurn
    (:0
      (Variables|Default|SetplayerTurn 1))
    (:1
      (Variables|Default|SetplayerTurn 0))))

(event Custom|MovePiece_GS
  (params (TileMovingTo :type String) (CurrentlySelectedTile :type Board%20Tile%20BP%20Object%20Reference))
  (CallFunction|MovePieceGSMulti TileMovingTo CurrentlySelectedTile))

(fn ConstructionScript
  (bind _outactors (Actor|GetAllActorsOfClass "/Game/Blueprints/Gameplay/BoardTile_BP.BoardTile_BP_C"))
  (Variables|Default|SetallBoardTiles _outactors))