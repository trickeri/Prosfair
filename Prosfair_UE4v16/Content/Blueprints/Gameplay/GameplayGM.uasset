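; GameplayGM is the gameplay game mode, handling player controller bookkeeping and session cleanup.
; It adds each new controller from OnSwapPlayerControllers to AllPlayerControllers.
; On logout, an exiting GameplayPC is passed to DestroySessionCaller on the game instance.
; RespawnPlayer is an empty stub; logic to gather PlayerStarts, then spawn and possess the selected character at a random one, is disconnected and never runs.
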(event Custom|RespawnPlayer
  (params (PlayerController :type Player%20Controller%20Object%20Reference) (PlayerCharacter :type Character%20Class%20Reference))
  ;[1 1 1] Spawn the player with their selected character from the Gameplay PC.
)

(event EventOnSwapPlayerControllers
  (params (OldPC :type Player%20Controller%20Object%20Reference) (NewPC :type Player%20Controller%20Object%20Reference))
  ;[1 1 1] Keeps track of connected player controllers.
  (Utilities|Array|Add (Variables|GameInfo|GetAllPlayerControllers) NewPC))

(event EventOnLogout
  (params (ExitingController :type Controller%20Object%20Reference))
  ;[1 1 1] Event OnLogout - Destroy session caller in game info instance.
  (bind _asgameplay_pc (Utilities|Casting|CastToGameplayPC ExitingController))
  (Default|DestroySessionCaller (.AsGame%20Info%20Instance (Utilities|Casting|CastToGameInfoInstance (Game|GetGameInstance))) _asgameplay_pc))

(fn ConstructionScript)