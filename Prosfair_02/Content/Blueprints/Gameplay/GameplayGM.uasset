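; GameplayGM is the gameplay game mode that spawns players as their selected characters and handles logouts.
; It records player controllers in an array when they are swapped in.
; Respawning destroys any current pawn, spawns the passed character class at a random PlayerStart and possesses it.
; On logout of a GameplayPC, it calls DestroySessionCaller on the GameInfoInstance game instance with that controller.
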(event Custom|RespawnPlayer
  (params (PlayerController :type Player%20Controller%20Object%20Reference) (PlayerCharacter :type Character%20Class%20Reference))
  (bind _returnvalue (Pawn|GetControlledPawn PlayerController))
  ;[1 1 1] Spawn the player with their selected character from the Gameplay PC.
  (bind _outactors (Actor|GetAllActorsOfClass "/Script/Engine.PlayerStart"))
  (Variables|GameInfo|SetSpawnPoints _outactors)
  (Utilities|IsValid _returnvalue
    (:Is%20Valid
      (Actor|DestroyActor _returnvalue))
    (:Is%20Not%20Valid
      _))
  (bind _returnvalue_2 (Game|SpawnActorfromClass PlayerCharacter (Transformation|GetActorTransform (Utilities|Array|Get(acopy) (Variables|GameInfo|GetSpawnPoints) (Math|Random|RandomIntegerinRange 0 (- (Utilities|Array|Length (Variables|GameInfo|GetSpawnPoints)) 1)))) "Undefined" 0 0))
  (Pawn|Possess PlayerController _returnvalue_2))

(event EventOnSwapPlayerControllers
  (params (OldPC :type Player%20Controller%20Object%20Reference) (NewPC :type Player%20Controller%20Object%20Reference))
  ;[1 1 1] Keeps track of connected player controllers.
  (Utilities|Array|Add (Variables|GameInfo|GetAllPlayerControllers) NewPC))

(event EventOnLogout
  (params (ExitingController :type Controller%20Object%20Reference))
  ;[1 1 1] Event OnLogout - Destroy session caller in game info instance.
  (bind _asgameplay_pc (Utilities|Casting|CastToGameplayPC ExitingController))
  (Default|DestroySessionCaller (.AsGame%20Info%20Instance (Utilities|Casting|CastToGameInfoInstance (Game|GetGameInstance))) _asgameplay_pc))

(fn ConstructionScript)