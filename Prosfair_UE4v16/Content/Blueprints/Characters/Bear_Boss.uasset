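; Bear boss character that loops through a timed walk, roar and attack cycle, with no targeting or damage logic.
; Chained custom events use delays, random for walking, and set walk and attack flags on BP_BearAnim to switch animations.
; While walking, Tick moves it forward a fixed step per frame without sweep.
; After each attack it sets a fixed absolute 180-degree rotation, then walks again.
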(event Custom|StartBearRoar
  (bind _asbp_bear_anim (Utilities|Casting|CastToBP_BearAnim (Components|SkeletalMesh|GetAnimInstance (Variables|Character|GetMesh))))
  (Variables|/Game/InfinityBladeAdversaries/Enemy/Enemy_Bear/BP_BearAnim.BP_BearAnim_C|SetisWalking _asbp_bear_anim false)
  (Variables|/Game/InfinityBladeAdversaries/Enemy/Enemy_Bear/BP_BearAnim.BP_BearAnim_C|SetisAttacking _asbp_bear_anim false)
  (Utilities|FlowControl|Delay 4.3)
  (CallFunction|StartBearAttack))

(event Custom|StartBearAttack
  (bind _asbp_bear_anim (Utilities|Casting|CastToBP_BearAnim (Components|SkeletalMesh|GetAnimInstance (Variables|Character|GetMesh))))
  (Variables|/Game/InfinityBladeAdversaries/Enemy/Enemy_Bear/BP_BearAnim.BP_BearAnim_C|SetisAttacking _asbp_bear_anim true)
  (Utilities|FlowControl|Delay 2.2)
  (Variables|/Game/InfinityBladeAdversaries/Enemy/Enemy_Bear/BP_BearAnim.BP_BearAnim_C|SetisAttacking _asbp_bear_anim false)
  (Transformation|SetActorRotation "0,180.000000, 0")
  (CallFunction|StartBearWalk))

(event Custom|StartBearWalk
  (bind _asbp_bear_anim (Utilities|Casting|CastToBP_BearAnim (Components|SkeletalMesh|GetAnimInstance (Variables|Character|GetMesh))))
  (Variables|/Game/InfinityBladeAdversaries/Enemy/Enemy_Bear/BP_BearAnim.BP_BearAnim_C|SetisWalking _asbp_bear_anim true)
  (Variables|Default|SetisWalking true)
  (Utilities|FlowControl|Delay (Math|Random|RandomFloatinRange 5.0 1e+01))
  (Variables|/Game/InfinityBladeAdversaries/Enemy/Enemy_Bear/BP_BearAnim.BP_BearAnim_C|SetisWalking _asbp_bear_anim false)
  (Variables|Default|SetisWalking false)
  (CallFunction|StartBearRoar))

(event EventBeginPlay
  (CallFunction|StartBearWalk))

(event EventTick
  (params (DeltaSeconds :type Float%20%28single-precision%29))
  (if (Variables|Default|GetisWalking)
    (Transformation|SetActorLocation (+ (Transformation|GetActorLocation) (* (Transformation|GetActorForwardVector) "4.000000,4.000000,4.000000")) false false)))

(fn ConstructionScript)